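; BP_GroundItem is an interactable item placed on the ground, with a viewer mesh that shows whether it can currently be interacted with.
; BeginPlay creates a dynamic material instance on InteractableViewer, starting red; OnInteractable turns its Color parameter green and OnNonInteractable turns it back to red.
; The construction script raises InteractionCollider by its box Z extent so it rests on the actor origin.
; Interact is a placeholder that only prints a debug string.
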(event EventOnInteractable
  (CallFunction|ChangeInteractableViewerColor "(R=0.000000,G=1.000000,B=0.000000,A=1.000000)"))

(event EventInteract
  (Development|PrintString "Interact" true true "(R=1.000000,G=0.000000,B=0.000000,A=1.000000)"))

(event EventOnNonInteractable
  (CallFunction|ChangeInteractableViewerColor "(R=1.000000,G=0.000000,B=0.000000,A=1.000000)"))

(event EventBeginPlay
  (CallFunction|CreateMaterialInteractableViewer))

(fn ConstructionScript
  (bind _interactioncollider (Variables|Default|GetInteractionCollider))
  (Transformation|SetRelativeLocation _interactioncollider (Math|Vector|MakeVector 0.0 0.0 (.z (Variables|/Script/Engine.BoxComponent|GetBoxExtent _interactioncollider))) false false))

(fn CreateMaterialInteractableViewer
  (bind _returnvalue (Rendering|Material|CreateDynamicMaterialInstance (Variables|Default|GetInteractableViewer) 0 (Rendering|Material|GetMaterial (Variables|Default|GetInteractableViewer) 0) "None" :!class /Script/Engine.PrimitiveComponent))
  (bind _output_get (Variables|Default|SetM_InteractableViewer _returnvalue))
  (Rendering|Material|SetVectorParameterValue _output_get "Color" "(R=1.000000,G=0.000000,B=0.000000,A=1.000000)" :!class /Script/Engine.MaterialInstanceDynamic))

(fn ChangeInteractableViewerColor
  (params (Value :type Linear%20Color%20Structure))
  (Rendering|Material|SetVectorParameterValue (Variables|Default|GetM_InteractableViewer) "Color" Value :!class /Script/Engine.MaterialInstanceDynamic))