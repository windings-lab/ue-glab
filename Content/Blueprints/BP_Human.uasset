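; Player-controlled human character with camera-relative movement, jumping, a walk speed toggle and interaction with nearby actors.
; An InteractableGraph binds the InteractionCollider's overlap events to refresh the list of candidates.
; Each Tick it targets the nearest candidate, messaging it and the previous target about interactability, and the Interact input messages the current target.
; BeginPlay also checks for a valid Ability System Component, only printing the result.
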(event EventBeginPlay
  (Variables|Default|SetJumpMaxHoldTime 0.0)
  (|InteractableGraph
    (:OutBeginPlay
      (Utilities|IsValid (Ability|GetAbilitySystemComponent 0)
        (:Is%20Valid
          (Development|PrintString "Valid ASC"))))))

(event EventTick
  (params (DeltaSeconds :type Float%20%28single-precision%29))
  (|InteractableGraph) ; enters at Tick
)

(event Input|EnhancedActionEvents|EnhancedInputActionIA_Move
  (params (ActionValue :type Vector%202D%20Structure) (ElapsedSeconds :type Float%20%28double-precision%29) (TriggeredSeconds :type Float%20%28double-precision%29) (InputAction :type Input%20Action%20Object%20Reference :default "/Game/Input/IA_Move.IA_Move"))
  (CallFunction|Move (.x ActionValue) (.y ActionValue)))

(event Input|EnhancedActionEvents|EnhancedInputActionIA_Jump
  (params (ActionValue :type Boolean) (ElapsedSeconds :type Float%20%28double-precision%29) (TriggeredSeconds :type Float%20%28double-precision%29) (InputAction :type Input%20Action%20Object%20Reference :default "/Game/Input/IA_Jump.IA_Jump"))
  (:Started
    (Character|Jump))
  (:Canceled
    (Character|StopJumping :!label _label))
  (:Completed
    (goto _label)))

(event Input|EnhancedActionEvents|EnhancedInputActionIA_Walk
  (params (ActionValue :type Boolean) (ElapsedSeconds :type Float%20%28double-precision%29) (TriggeredSeconds :type Float%20%28double-precision%29) (InputAction :type Input%20Action%20Object%20Reference :default "/Game/Input/IA_Walk.IA_Walk"))
  (CallFunction|ToggleWalk))

(event Input|EnhancedActionEvents|EnhancedInputActionIA_Interact
  (params (ActionValue :type Boolean) (ElapsedSeconds :type Float%20%28double-precision%29) (TriggeredSeconds :type Float%20%28double-precision%29) (InputAction :type Input%20Action%20Object%20Reference :default "/Game/Input/IA_Interact.IA_Interact"))
  (Interactables|Interact))

(fn ConstructionScript)

(fn HandleInteractable
  (bind _interactablelist (Variables|Interactables|GetInteractableList))
  (if (Utilities|Array|IsNotEmpty _interactablelist)
    (Utilities|IsValid (Variables|Interactables|GetInteractable)
      (:Is%20Valid
        (Class|BPIInteractable|OnNonInteractable(Message) (Variables|Interactables|GetInteractable)))
      (:Is%20Not%20Valid
        _))
    (bind _output_get (Variables|Interactables|SetInteractable (.ReturnValue (Actor|FindNearestActor (Transformation|GetActorLocation) _interactablelist))))
    (Class|BPIInteractable|OnInteractable(Message) _output_get)
    (else
      (Utilities|IsValid (Variables|Interactables|GetInteractable)
        (:Is%20Valid
          (Class|BPIInteractable|OnNonInteractable(Message) (Variables|Interactables|GetInteractable))
          (Variables|Interactables|SetInteractable 0))))))

(fn GetOverlappedInteractables
  (Variables|Interactables|SetInteractableList (Collision|GetOverlappingActors (Variables|Default|GetInteractionCollider) 0 :!class /Script/Engine.PrimitiveComponent)))

(fn Interact
  (bind _interactable (Variables|Interactables|GetInteractable))
  (Utilities|IsValid _interactable
    (:Is%20Valid
      (Class|BPIInteractable|Interact(Message) _interactable))))

(fn ToggleWalk
  (bind _charactermovement (Variables|Character|GetCharacterMovement))
  (Utilities|FlowControl|FlipFlop
    (:A
      (Variables|/Script/Engine.CharacterMovementComponent|SetMaxWalkSpeed _charactermovement 3e+02))
    (:B
      (Variables|/Script/Engine.CharacterMovementComponent|SetMaxWalkSpeed _charactermovement 6e+02))))

(fn Move
  (params (B :type Float%20%28double-precision%29) (A :type Float%20%28double-precision%29))
  (bind _returnvalue (Pawn|GetControlRotation :!class /Script/Engine.Pawn))
  (Class|PawnMovementComponent|AddInputVector (Variables|Character|GetCharacterMovement) (* (Math|Vector|GetForwardVector (Math|Rotator|MakeRotator (.roll _returnvalue) 0.0 (.yaw _returnvalue))) B) false)
  (Class|PawnMovementComponent|AddInputVector (Variables|Character|GetCharacterMovement) (* A (Math|Vector|GetRightVector (Math|Rotator|MakeRotator (.roll _returnvalue) 0.0 (.yaw _returnvalue)))) false))

(event Custom|OnFoundInteractable
  (params (OverlappedComponent :type Primitive%20Component%20Object%20Reference) (OtherActor :type Actor%20Object%20Reference) (OtherComp :type Primitive%20Component%20Object%20Reference) (OtherBodyIndex :type Integer) (bFromSweep :type Boolean) (SweepResult :type Hit%20Result%20Structure%20%28by%20ref%29))
  (Interactables|GetOverlappedInteractables))

(event Custom|OnInteractableOutOfReach
  (params (OverlappedComponent :type Primitive%20Component%20Object%20Reference) (OtherActor :type Actor%20Object%20Reference) (OtherComp :type Primitive%20Component%20Object%20Reference) (OtherBodyIndex :type Integer))
  (Interactables|GetOverlappedInteractables))