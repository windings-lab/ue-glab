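; BP_HumanDebug_AC is an actor component that shows on-screen movement debug info for a BP_Human owner.
; On BeginPlay it casts its owner to BP_Human and caches the reference.
; Each tick it prints the CharacterMovement velocity length as speed and the current movement mode, using keyed PrintText calls so each readout has its own key.
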(event EventBeginPlay
  (bind _asbp_human (Utilities|Casting|CastToBP_Human (Components|GetOwner)))
  (Variables|Default|SetOwner_Human _asbp_human))

(event EventTick
  (params (DeltaSeconds :type Float%20%28single-precision%29))
  (CallFunction|PrintSpeed)
  (Development|PrintText (Utilities|Text|FormatText "Movement Mode: {MM}" (|GenerictoText (Variables|/Script/Engine.CharacterMovementComponent|GetMovementMode (Variables|/Script/Engine.Character|GetCharacterMovement (Variables|Default|GetOwner_Human))))) true true "(R=0.000000,G=0.660000,B=1.000000,A=1.000000)" 2.0 "MMDebug"))

(fn PrintSpeed
  (Development|PrintText (Utilities|Text|FormatText "Speed: {Speed}" (Math|Vector|VectorLength (Variables|/Script/Engine.MovementComponent|GetVelocity (Variables|/Script/Engine.Character|GetCharacterMovement (Variables|Default|GetOwner_Human))))) true true "(R=0.000000,G=0.660000,B=1.000000,A=1.000000)" 2.0 "SpeedDebug"))